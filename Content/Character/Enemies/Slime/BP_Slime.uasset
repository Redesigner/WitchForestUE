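; Slime enemy Blueprint that gets knocked back when damaged and displays its health on a healthbar widget.
; On BeginPlay it binds a damage handler that applies a movement impulse against the hit normal with an upward lift.
; Each Tick it polls an Ability System attribute and writes it to the healthbar as a fraction, assuming a fixed maximum of 100.
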(event Custom|OnTakeDamage_Event
  (params (Source :type Actor%20Object%20Reference) (Hit :type Hit%20Result%20Structure))
  (Class|EnemyMovementComponent|AddImpulse (Variables|Default|GetMovementComponent) (+ (* (.Normal (Collision|BreakHitResult Hit)) -5e+02) "0.000000,0.000000,300.000000")))

(event EventBeginPlay
  (EventDispatchers|AssignOnTakeDamage (delegate Custom|OnTakeDamage_Event)))

(event EventTick
  (params (DeltaSeconds :type Float%20%28single-precision%29))
  (bind _aswbp_healthbar (Utilities|Casting|CastToWBP_Healthbar (UserInterface|GetWidget (Variables|Default|GetHealthbar))))
  (Variables|/Game/UI/WBP_Healthbar.WBP_Healthbar_C|SetHealthPercentage _aswbp_healthbar (/ (.ReturnValue (Ability|Attribute|GetFloatAttributefromAbilitySystemComponent (Variables|Default|GetAbilitySystem) "(AttributeName=\"Health\",Attribute=/Script/WitchForestAbility.BaseAttributeSet:Health,AttributeOwner=\"/Script/CoreUObject.Class'/Script/WitchForestAbility.BaseAttributeSet'\")")) 1e+02)))

(fn ConstructionScript)