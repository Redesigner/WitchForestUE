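; BP_SlimeAggressive is an aggressive slime enemy Blueprint that reacts visually and physically to being damaged.
; Taking damage applies an impulse through its movement component, based on the hit normal plus an upward boost, to knock it back.
; A GameplayCue.Damage event briefly flashes the mesh's glow material parameter, cleared by a timer.
; Each tick, it copies an Ability System attribute into its healthbar widget as a fraction.
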(event Custom|End%20DamageEffect
  (Rendering|Material|SetScalarParameterValueonMaterials (Variables|Character|GetMesh) "GlowAmount" 0.0))

(event Custom|OnTakeDamage_Event
  (params (Source :type Actor%20Object%20Reference) (Hit :type Hit%20Result%20Structure))
  (Class|EnemyMovementComponent|AddImpulse (Variables|Default|GetMovementComponent) (+ (* (.Normal (Collision|BreakHitResult Hit)) -5e+02) "0.000000,0.000000,300.000000")))

(event EventBeginPlay
  (EventDispatchers|AssignOnTakeDamage (delegate Custom|OnTakeDamage_Event)))

(event EventTick
  (params (DeltaSeconds :type Float%20%28single-precision%29))
  (bind _aswbp_healthbar (Utilities|Casting|CastToWBP_Healthbar (UserInterface|GetWidget (Variables|Default|GetHealthbar))))
  (Variables|/Game/UI/WBP_Healthbar.WBP_Healthbar_C|SetHealthPercentage _aswbp_healthbar (/ (.ReturnValue (Ability|Attribute|GetFloatAttributefromAbilitySystemComponent (Variables|Default|GetAbilitySystem) "(AttributeName=\"Health\",Attribute=/Script/WitchForestAbility.BaseAttributeSet:Health,AttributeOwner=\"/Script/CoreUObject.Class'/Script/WitchForestAbility.BaseAttributeSet'\")")) 1e+02)))

(event EventGameplayCue.Damage
  (params (EventType :type EGameplayCueEvent%20Enum :default "OnActive") (Parameters :type Gameplay%20Cue%20Parameters%20Structure%20%28by%20ref%29))
  (switch Utilities|FlowControl|Switch|SwitchonEGameplayCueEvent EventType
    (:Executed
      (Rendering|Material|SetScalarParameterValueonMaterials (Variables|Character|GetMesh) "GlowAmount" 1.0)
      (Utilities|Time|SetTimerbyEvent (delegate Custom|End%20DamageEffect) 0.1))))

(fn ConstructionScript)