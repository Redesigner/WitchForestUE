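; Slime enemy character that gets knocked back when it takes damage.
; On BeginPlay it binds a handler to its OnTakeDamage event.
; The handler ignores damage whose source is the slime itself, otherwise applying a velocity-change impulse through CharacterMovement, directed against the hit normal with an added upward lift.
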(event Custom|OnTakeDamage_Event
  (params (Source :type Actor%20Object%20Reference) (Hit :type Hit%20Result%20Structure))
  (if (!= Source self)
    (Physics|AddImpulse (Variables|Character|GetCharacterMovement) (+ (* (.Normal (Collision|BreakHitResult Hit)) -5e+02) "0.000000,0.000000,300.000000") true)))

(event EventBeginPlay
  (Utilities|FlowControl|Sequence
    (:then_0
      (EventDispatchers|AssignOnTakeDamage (delegate Custom|OnTakeDamage_Event)))))

(event EventTick
  (params (DeltaSeconds :type Float%20%28single-precision%29)))

(event Collision|EventActorBeginOverlap
  (params (OtherActor :type Actor%20Object%20Reference)))

(fn ConstructionScript)