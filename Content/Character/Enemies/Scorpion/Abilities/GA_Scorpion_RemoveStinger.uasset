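; Gameplay ability that temporarily removes the scorpion enemy's stinger for a fixed delay.
; On activation it clears the HasTail flag on both the owner's blackboard and BP_Scorpion, then commits the ability.
; When the delay task finishes, it sets both flags back to true and ends the ability.
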(event Ability|EventActivateAbility
  (bind _returnvalue (Utilities|Name|MakeLiteralName "HasTail"))
  (bind _asbp_scorpion (Utilities|Casting|CastToBP_Scorpion (Ability|GetOwningActorfromActorInfo)))
  (bind _returnvalue_2 (Class|WitchForestGameplayAbility|GetOwnerBlackboard)
    (:True
      (AI|Components|Blackboard|SetValueasBool _returnvalue_2 _returnvalue false)
      (Variables|/Game/Character/Enemies/Scorpion/BP_Scorpion.BP_Scorpion_C|SetHasTail _asbp_scorpion false)
      (Ability|CommitAbility)
      (GameplayTasks|TaskWaitDelay 0 15.0
        (:OnFinish
          (AI|Components|Blackboard|SetValueasBool _returnvalue_2 _returnvalue true)
          (Variables|/Game/Character/Enemies/Scorpion/BP_Scorpion.BP_Scorpion_C|SetHasTail _asbp_scorpion true)
          (Ability|EndAbility))))))