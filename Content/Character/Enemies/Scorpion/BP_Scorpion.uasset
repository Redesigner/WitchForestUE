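; Scorpion enemy character whose stinger tail can be harvested by interaction.
; A TailFired gameplay cue hides the stinger mesh while active and restores it on removal.
; Damage from any source but itself knocks it back along the hit normal with an upward pop.
; A timed hold interaction, allowed only while immobile with a tail, spawns a stinger pickup and sends itself a RemoveStinger ability trigger event.
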(event Custom|OnTakeDamage_Event
  (params (Source :type Actor%20Object%20Reference) (Hit :type Hit%20Result%20Structure))
  (if (!= Source self)
    (Physics|AddImpulse (Variables|Character|GetCharacterMovement) (+ (* (.Normal (Collision|BreakHitResult Hit)) -5e+02) "0.000000,0.000000,300.000000") true)))

(event EventBeginPlay
  (Utilities|FlowControl|Sequence
    (:then_0
      (EventDispatchers|AssignOnTakeDamage (delegate Custom|OnTakeDamage_Event)))))

(event EventInteract
  (params (Source :type Actor%20Object%20Reference))
  (Game|SpawnActorfromClass "/Game/Dynamic/Pickups/Ingredients/StingerTail/BP_Pickup_StingerTail.BP_Pickup_StingerTail_C" (Math|Transform|MakeTransform (Transformation|GetWorldLocation (Variables|Default|GetInteractionSphere)) (Transformation|GetActorRotation)) "AdjustIfPossibleButAlwaysSpawn" "MultiplyWithRoot" 0 self)
  (Ability|SendGameplayEventtoActor self "(TagName=\"GameplayEvent.AbilityTrigger.Scorpion.RemoveStinger\")"))

(event EventTick
  (params (DeltaSeconds :type Float%20%28single-precision%29)))

(event Collision|EventActorBeginOverlap
  (params (OtherActor :type Actor%20Object%20Reference)))

(event EventGameplayCue.Enemies.Scorpion.TailFired
  (params (EventType :type EGameplayCueEvent%20Enum :default "OnActive") (Parameters :type Gameplay%20Cue%20Parameters%20Structure%20%28by%20ref%29))
  (bind _stingermesh (Variables|Default|GetStingerMesh))
  (switch Utilities|FlowControl|Switch|SwitchonEGameplayCueEvent EventType
    (:OnActive
      (Rendering|SetVisibility _stingermesh false false))
    (:Removed
      (Rendering|SetVisibility _stingermesh true false))))

(fn ConstructionScript)

(fn CanInteract
  (params (Source :type Actor%20Object%20Reference))
  (return (and (GameplayTags|HasMatchingGameplayTag (Variables|Default|GetAbilitySystem) "(TagName=\"GameplayEffect.Immobile\")") (Variables|Default|GetHasTail))))

(fn GetRequiredHoldTime
  (return 2.0))