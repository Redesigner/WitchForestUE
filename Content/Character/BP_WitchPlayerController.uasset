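; Player controller for the witch character that builds the player's HUD when SetupUI fires with the player state.
; It adds a health widget whose view model binds to the player's WitchForest ability system component and attribute set.
; It also adds a hotbar whose four inventory view models each bind to one slot of the main item set in the player state's inventory component.
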(event EventSetupUI
  (params (WitchPlayerState :type Witch%20Player%20State%20Object%20Reference))
  (bind _returnvalue (Actor|GetComponentbyClass WitchPlayerState "/Script/WitchForestGame.InventoryComponent"))
  (Utilities|FlowControl|Sequence
    (:then_0
      (bind _returnvalue_2 (UserInterface|CreateWidget "/Game/UI/WBP_PlayerHealth.WBP_PlayerHealth_C"))
      (UserInterface|Viewport|AddtoViewport _returnvalue_2 0)
      (bind _aswitch_forest_asc (Utilities|Casting|CastToWitchForestASC (Ability|GetAbilitySystemComponent WitchPlayerState)))
      (bind _output_get (Variables|Default|SetWitch%20Player%20State WitchPlayerState))
      (Class|HealthViewModel|BindAttributeSet (Variables|/Game/UI/WBP_PlayerHealth.WBP_PlayerHealth_C|GetHealthViewModel _returnvalue_2) _aswitch_forest_asc (Class|WitchPlayerState|GetAttributeSet _output_get)))
    (:then_1
      (bind _returnvalue_3 (UserInterface|CreateWidget "/Game/UI/WBP_Hotbar.WBP_Hotbar_C"))
      (UserInterface|Viewport|AddtoViewport _returnvalue_3 0)
      (Utilities|FlowControl|Sequence
        (:then_0
          (Class|InventoryViewModel|BindInventory (Variables|/Game/UI/WBP_Hotbar.WBP_Hotbar_C|GetInventoryViewModel _returnvalue_3) _returnvalue "/Game/Dynamic/Pickups/ItemSet_Main.ItemSet_Main"))
        (:then_1
          (Class|InventoryViewModel|BindInventory (Variables|/Game/UI/WBP_Hotbar.WBP_Hotbar_C|GetInventoryViewModel_1 _returnvalue_3) _returnvalue "/Game/Dynamic/Pickups/ItemSet_Main.ItemSet_Main" 1))
        (:then_2
          (Class|InventoryViewModel|BindInventory (Variables|/Game/UI/WBP_Hotbar.WBP_Hotbar_C|GetInventoryViewModel_2 _returnvalue_3) _returnvalue "/Game/Dynamic/Pickups/ItemSet_Main.ItemSet_Main" 2))
        (:then_3
          (Class|InventoryViewModel|BindInventory (Variables|/Game/UI/WBP_Hotbar.WBP_Hotbar_C|GetInventoryViewModel_3 _returnvalue_3) _returnvalue "/Game/Dynamic/Pickups/ItemSet_Main.ItemSet_Main" 3))))))

(fn ConstructionScript)