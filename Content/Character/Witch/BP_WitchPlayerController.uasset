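; Player controller for the Witch character that builds the player's HUD and shows recipe-discovered notifications.
; SetupUI creates health, hotbar and controller-hint widgets and binds their view models to the player state's attribute set, inventory and ability system (MVVM style).
; Each hotbar slot binds its own view model to an index of the main item set, and control tips watch selected ability input tags.
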(event EventDisplayRecipeDiscoveredMessage
  (params (Recipe :type Potion%20Recipe%20Structure) (Data :type Inventory%20Item%20Data%20Structure))
  (bind _returnvalue (UserInterface|CreateWidget "/Game/UI/Notifications/WBP_Notification_RecipeLearned1.WBP_Notification_RecipeLearned1_C" self))
  (UserInterface|Viewport|AddtoViewport _returnvalue 5)
  (Variables|Default|SetNotificationWidget _returnvalue)
  (Default|SetItemData _returnvalue Data))

(event EventSetupUI
  (params (WitchPlayerState :type Witch%20Player%20State%20Object%20Reference))
  (bind _returnvalue (Actor|GetComponentbyClass WitchPlayerState "/Script/WitchForestGame.InventoryComponent"))
  (Utilities|FlowControl|Sequence
    (:then_0
      (bind _returnvalue_2 (UserInterface|CreateWidget "/Game/UI/WBP_PlayerHealth.WBP_PlayerHealth_C"))
      (UserInterface|Viewport|AddtoViewport _returnvalue_2 0)
      (bind _aswitch_forest_asc (Utilities|Casting|CastToWitchForestASC (Ability|GetAbilitySystemComponent WitchPlayerState)))
      (bind _output_get (Variables|Default|SetWitch%20Player%20State WitchPlayerState))
      (Utilities|IsValid (Class|WitchPlayerState|GetAttributeSet _output_get)
        (:Is%20Valid
          (Class|HealthViewModel|BindAttributeSet (Variables|/Game/UI/WBP_PlayerHealth.WBP_PlayerHealth_C|GetHealthViewModel _returnvalue_2) _aswitch_forest_asc (Class|WitchPlayerState|GetAttributeSet _output_get)))))
    (:then_1
      (bind _returnvalue_3 (UserInterface|CreateWidget "/Game/UI/WBP_Hotbar.WBP_Hotbar_C"))
      (UserInterface|Viewport|AddtoViewport _returnvalue_3 0)
      (Utilities|FlowControl|Sequence
        (:then_0
          (Class|InventoryViewModel|BindInventory (Variables|/Game/UI/WBP_Hotbar.WBP_Hotbar_C|GetInventoryViewModel _returnvalue_3) _returnvalue "/Game/Dynamic/Pickups/ItemSet_Main.ItemSet_Main"))
        (:then_1
          (Class|InventoryViewModel|BindInventory (Variables|/Game/UI/WBP_Hotbar.WBP_Hotbar_C|GetInventoryViewModel_1 _returnvalue_3) _returnvalue "/Game/Dynamic/Pickups/ItemSet_Main.ItemSet_Main" 1))
        (:then_2
          (Class|InventoryViewModel|BindInventory (Variables|/Game/UI/WBP_Hotbar.WBP_Hotbar_C|GetInventoryViewModel_2 _returnvalue_3) _returnvalue "/Game/Dynamic/Pickups/ItemSet_Main.ItemSet_Main" 2))
        (:then_3
          (Class|InventoryViewModel|BindInventory (Variables|/Game/UI/WBP_Hotbar.WBP_Hotbar_C|GetInventoryViewModel_3 _returnvalue_3) _returnvalue "/Game/Dynamic/Pickups/ItemSet_Main.ItemSet_Main" 3))))
    (:then_2
      (bind _returnvalue_4 (UserInterface|CreateWidget "/Game/UI/WBP_ControllerHints.WBP_ControllerHints_C"))
      (UserInterface|Viewport|AddtoViewport _returnvalue_4 0)
      (Class|ControlTipsViewModel|BindAbilitySystem (Variables|/Game/UI/WBP_ControllerHints.WBP_ControllerHints_C|GetControlTipsViewModel _returnvalue_4) (Class|WitchPlayerController|GetWitchForestASC) self (Utilities|Array|MakeArray "(TagName=\"InputTag.Ability.PrimarySpell\")" "(TagName=\"InputTag.Ability.PickupThrow\")" "(TagName=\"InputTag.Ability.StoreWithdraw\")"))
      (Class|ControlTipsViewModel|SetInputHints (Variables|/Game/UI/WBP_ControllerHints.WBP_ControllerHints_C|GetControlTipsViewModel _returnvalue_4) "/Game/UI/Buttons/InputHints_Default.InputHints_Default"))))

(fn ConstructionScript)