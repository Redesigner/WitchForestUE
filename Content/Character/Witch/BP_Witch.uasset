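; Witch character Blueprint that handles player coloring, a gameplay effect display and healing feedback.
; On BeginPlay it puts a dynamic hat material instance on the placeholder mesh, which SetPlayerColor later tints through a color parameter.
; On possession it creates an effect list widget for EffectDisplay and binds its view model to the character's Ability System Component.
; The GameplayCue.Heal event spawns an attached healing particle system on the capsule when executed.
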(event EventBeginPlay
  (bind _returnvalue (Rendering|Material|CreateDynamicMaterialInstance "/Game/Character/Witch/Materials/MI_Witch_Hat2.MI_Witch_Hat2" "None" "None" :!class /Script/Engine.KismetMaterialLibrary))
  (bind _output_get (Variables|Default|SetPlayer%20Color%20Material _returnvalue))
  (Rendering|Material|SetMaterial (Variables|Default|GetPlaceholderMesh) 0 _output_get))

(event EventPossessed
  (params (NewController :type Controller%20Object%20Reference))
  (bind _returnvalue (UserInterface|CreateWidget "/Game/UI/World/GameplayEffectDisplay/WBP_GameplayEffectList.WBP_GameplayEffectList_C"))
  (UserInterface|SetWidget (Variables|Default|GetEffectDisplay) _returnvalue)
  (Class|EffectDisplayViewModel|BindAbilitySystemComponent (Variables|/Game/UI/World/GameplayEffectDisplay/WBP_GameplayEffectList.WBP_GameplayEffectList_C|GetEffectDisplayViewModel _returnvalue) (Ability|GetAbilitySystemComponent 0)))

(event EventSetPlayerColor
  (params (Color :type Color%20Structure))
  (bind _player_color_material (Variables|Default|GetPlayer%20Color%20Material))
  (Utilities|IsValid _player_color_material
    (:Is%20Valid
      (Rendering|Material|SetVectorParameterValue _player_color_material "Base Color" (Math|Conversions|ToLinearColor(Color) Color) :!class /Script/Engine.MaterialInstanceDynamic))))

(event EventGameplayCue.Heal
  (params (EventType :type EGameplayCueEvent%20Enum :default "OnActive") (Parameters :type Gameplay%20Cue%20Parameters%20Structure%20%28by%20ref%29))
  (switch Utilities|FlowControl|Switch|SwitchonEGameplayCueEvent EventType
    (:Executed
      (Niagara|SpawnSystemAttached "/Game/Particles/NS_Healing.NS_Healing" (Variables|Default|GetCapsuleComponent) "None" "0.000000,0.000000,50.000000" "0, 0, 0" "SnapToTarget" false))))

(fn ConstructionScript)