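; BP_SimpleLockedDoor is a world door with a lock mesh, reacting to unlock, open and close events.
; Unlocking destroys the lock mesh component if it is valid.
; Opening hides the door mesh and disables its collision instead of animating it.
; Closing restores query and physics collision, but the node that would make the mesh visible again is disconnected.
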(event EventOnOpened
  (bind _doormesh (Variables|Default|GetDoorMesh))
  (Collision|SetCollisionEnabled _doormesh "NoCollision")
  (Rendering|SetVisibility _doormesh false false))

(event EventOnClosed
  (Collision|SetCollisionEnabled (Variables|Default|GetDoorMesh) "QueryAndPhysics"))

(event EventOnUnlocked
  (bind _lockmesh (Variables|Default|GetLockMesh))
  (Utilities|IsValid _lockmesh
    (:Is%20Valid
      (Components|DestroyComponent _lockmesh))))

(fn ConstructionScript)